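; Gnomeo is a gnome target actor that awards the player a single point when hit by a DrugBaseBP actor.
; Its Sphere plays a "woo" sound on overlap, re-armed when an overlap ends.
; Every drug hit destroys the drug, but only the first spawns an impact effect and fires its own PointGained dispatcher.
; That handler increments FirstPersonCharacter's PointsCount, plays Audio and reveals the initially hidden component A.
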(event OnComponentBeginOverlap(Sphere)
  (params (OverlappedComponent :type Primitive%20Component%20Object%20Reference) (OtherActor :type Actor%20Object%20Reference) (OtherComp :type Primitive%20Component%20Object%20Reference) (OtherBodyIndex :type Integer) (bFromSweep :type Boolean) (SweepResult :type Hit%20Result%20Structure%20%28by%20ref%29))
  (Utilities|FlowControl|DoOnce false
    (:Completed
      (Audio|PlaySoundatLocation "/Game/Sound/Character/Gnome-woo_Cue.Gnome-woo_Cue" (Transformation|GetWorldLocation (Variables|Default|GetGnomeo)) "0, 0, 0" 1.0 1.0 0.0 0 0 0))))

(event OnComponentEndOverlap(Sphere)
  (params (OverlappedComponent :type Primitive%20Component%20Object%20Reference) (OtherActor :type Actor%20Object%20Reference) (OtherComp :type Primitive%20Component%20Object%20Reference) (OtherBodyIndex :type Integer))
  (Utilities|FlowControl|DoOnce false) ; enters at Reset
)

(event OnComponentHit(Sphere)
  (params (HitComponent :type Primitive%20Component%20Object%20Reference) (OtherActor :type Actor%20Object%20Reference) (OtherComp :type Primitive%20Component%20Object%20Reference) (NormalImpulse :type Vector :default "0, 0, 0") (Hit :type Hit%20Result%20Structure%20%28by%20ref%29))
  (bind (_bblockinghit _binitialoverlap _time _distance _location _impactpoint _normal _impactnormal) (Collision|BreakHitResult Hit))
  (bind _asdrug_base_bp (Utilities|Casting|CastToDrugBaseBP OtherActor))
  (if (== _asdrug_base_bp OtherActor)
    (Actor|DestroyActor _asdrug_base_bp)
    (Utilities|FlowControl|DoOnce false
      (:Completed
        (Niagara|SpawnSystematLocation "/Game/Effects/HitEffect.HitEffect" _impactpoint (Math|Conversions|RotationFromXVector _impactnormal))
        (Default|CallPointGained)))))

(event Custom|OnPointGained
  (bind _asfirst_person_character (Utilities|Casting|CastToFirstPersonCharacter (Game|GetPlayerCharacter 0)))
  (Utilities|FlowControl|DoOnce false
    (:Completed
      (Math|Integer|IncrementInt (Variables|/Game/FirstPersonBP/Blueprints/FirstPersonCharacter.FirstPersonCharacter_C|GetPointsCount _asfirst_person_character)
        (:%20%20
          (Audio|Components|Audio|Play (Variables|Default|GetAudio) 0.0)
          (Rendering|SetVisibility (Variables|Default|Geta) true false))))))

(event EventBeginPlay
  (EventDispatchers|BindEventtoPointGained (delegate Custom|OnPointGained))
  (Rendering|SetVisibility (Variables|Default|Geta) false false))

(fn ConstructionScript)