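; DruggyPawnBP is a pawn that awards the player a point when a drug hits it.
; A capsule hit matching DrugBaseBP destroys the hit result's actor and calls the PointGained dispatcher, which the pawn binds to itself on BeginPlay.
; The handler increments PointsCount on FirstPersonCharacter and plays audio, behind a DoOnce that is never reset, so each pawn scores only once.
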(event OnComponentHit(Capsule)
  (params (HitComponent :type Primitive%20Component%20Object%20Reference) (OtherActor :type Actor%20Object%20Reference) (OtherComp :type Primitive%20Component%20Object%20Reference) (NormalImpulse :type Vector :default "0, 0, 0") (Hit :type Hit%20Result%20Structure%20%28by%20ref%29))
  (if (== OtherActor "/Game/Drugs/DrugBaseBP.DrugBaseBP")
    (Actor|DestroyActor (.HitActor (Collision|BreakHitResult Hit)))
    (Default|CallPointGained)))

(event Custom|OnPointGained
  (bind _asfirst_person_character (Utilities|Casting|CastToFirstPersonCharacter (Game|GetPlayerCharacter 0)))
  (Utilities|FlowControl|DoOnce false
    (:Completed
      (Math|Integer|IncrementInt (Variables|/Game/FirstPersonBP/Blueprints/FirstPersonCharacter.FirstPersonCharacter_C|GetPointsCount _asfirst_person_character)
        (:%20%20
          (Audio|Components|Audio|Play (Variables|Default|GetAudio) 0.0))))))

(event EventBeginPlay
  (EventDispatchers|BindEventtoPointGained (delegate Custom|OnPointGained)))

(fn ConstructionScript)